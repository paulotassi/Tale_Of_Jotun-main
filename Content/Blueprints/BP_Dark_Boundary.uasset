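; BP_Dark_Boundary is a trigger-zone actor that raises the player's Dark stat on entry.
; When a BP_ThirdPersonCharacter overlaps TriggerZone, it sets InZone and calls IncreaseDark on that character's BPCPlayerStats component.
; Leaving clears InZone and starts a delay with nothing after it; DecreaseDark and a repeating damage loop exist but are unwired.
; BeginPlay also caches stats from its owner, if that is the character.
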(event `self.ReceiveBeginPlay`
  (bind _asbp_third_person_character (cast `/Game/ThirdPerson/Blueprints/BP_ThirdPersonCharacter` (`self.GetOwner`)))
  (set `self.BPC Player Stats` (`/Game/ThirdPerson/Blueprints/BP_ThirdPersonCharacter.BPC_PlayerStats` _asbp_third_person_character)))

(event `self.TriggerZone.OnComponentBeginOverlap`
  (params (OverlappedComponent :type "PrimitiveComponent Object Reference") (OtherActor :type "Actor Object Reference") (OtherComp :type "PrimitiveComponent Object Reference") (OtherBodyIndex :type Integer) (bFromSweep :type Boolean) (SweepResult :type "HitResult Structure (by ref)"))
  (bind _asbp_third_person_character (cast `/Game/ThirdPerson/Blueprints/BP_ThirdPersonCharacter` OtherActor))
  (set `self.As BP Third Person Character` _asbp_third_person_character)
  (set `self.InZone?` true)
  (`/Game/Blueprints/BPC_PlayerStats.IncreaseDark` (`/Game/ThirdPerson/Blueprints/BP_ThirdPersonCharacter.BPC_PlayerStats` (`self.As BP Third Person Character`)) 10.0))

(event `self.TriggerZone.OnComponentEndOverlap`
  (params (OverlappedComponent :type "PrimitiveComponent Object Reference") (OtherActor :type "Actor Object Reference") (OtherComp :type "PrimitiveComponent Object Reference") (OtherBodyIndex :type Integer))
  (cast `/Game/ThirdPerson/Blueprints/BP_ThirdPersonCharacter` OtherActor)
  (set `self.InZone?` false)
  (`KismetSystemLibrary.Delay` 5.0))

(fn `UserConstructionScript`)