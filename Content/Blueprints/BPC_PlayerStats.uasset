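; Stats component for the player, dummy and AI that tracks health, stamina, XP, level and Dark, and updates their UI.
; BeginPlay waits a tick, then identifies the owner by cast to set CharacterType, which selects the health widget.
; Decrease functions report depletion, increases write only to the player HUD, and full XP triggers a level-up with sound.
; Dark's max clamp is unwired, and DecreaseDark and IncreaseMaxDark are empty.
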(event `self.ReceiveBeginPlay`
  (`KismetSystemLibrary.DelayUntilNextTick`)
  (bind _asbp_third_person_character (cast `/Game/ThirdPerson/Blueprints/BP_ThirdPersonCharacter` (`self.GetOwner`))
    (:`then`
      (set `self.Player Character BP` _asbp_third_person_character)
      (set `self.IsPlayer?` true)
      ;[1 1 1] Stamina
      (`ProgressBar.SetPercent` (`/Game/Ui/MainHud.StaminaBar` (`/Game/ThirdPerson/Blueprints/BP_ThirdPersonCharacter.HudWidget` (`self.Player Character BP`))) (/ (`self.CurrentStamina`) (`self.MaxStamina`)))
      ;[1 1 1] Health
      (set `self.CharacterType` "NewEnumerator0"))
    (:`CastFailed`
      (bind _asbp_dummy (cast `/Game/Blueprints/BP_Dummy` (`self.GetOwner`))
        (:`then`
          (set `self.Dummy Blueprint` _asbp_dummy)
          (set `self.IsPlayer?` false)
          (set `self.CharacterType` "NewEnumerator1"))
        (:`CastFailed`
          (bind _asbp_ai (cast `/Game/AI/BP_AI` (`self.GetOwner`)))
          (set `self.BP AI` _asbp_ai)
          (set `self.CharacterType` "NewEnumerator2")))))
  (`ProgressBar.SetPercent` (select `/Game/Blueprints/E_CharacterTypes` (`self.CharacterType`) :`NewEnumerator0` (`/Game/Ui/MainHud.HealthBar` (`/Game/ThirdPerson/Blueprints/BP_ThirdPersonCharacter.HudWidget` (`self.Player Character BP`))) :`NewEnumerator1` (`/Game/Ui/WB_DummyHealthbar.HealthBar` (`/Game/Blueprints/BP_Dummy.Widget Health Ui` (`self.Dummy Blueprint`))) :`NewEnumerator2` (`/Game/Ui/WB_DummyHealthbar.HealthBar` (`/Game/AI/BP_AI.Widget Health Ui` (`self.BP AI`)))) (/ (`self.CurrentHealth`) (`self.MaxHealth`)))
  (`TextBlock.SetText` (select `/Game/Blueprints/E_CharacterTypes` (`self.CharacterType`) :`NewEnumerator0` (`/Game/Ui/MainHud.HealthText` (`/Game/ThirdPerson/Blueprints/BP_ThirdPersonCharacter.HudWidget` (`self.Player Character BP`))) :`NewEnumerator1` (`/Game/Ui/WB_DummyHealthbar.HealthText` (`/Game/Blueprints/BP_Dummy.Widget Health Ui` (`self.Dummy Blueprint`))) :`NewEnumerator2` (`/Game/Ui/WB_DummyHealthbar.HealthText` (`/Game/AI/BP_AI.Widget Health Ui` (`self.BP AI`)))) (`KismetTextLibrary.Conv_DoubleToText` (`self.CurrentHealth`) "HalfToEven"))
  (if (`self.IsPlayer?`)
    ;[1 1 1] Xp
    (`ProgressBar.SetPercent` (`/Game/Ui/MainHud.XPProgressBar` (`/Game/ThirdPerson/Blueprints/BP_ThirdPersonCharacter.HudWidget` (`self.Player Character BP`))) (/ (`self.XP`) (`self.MaxXP`)))
    (`TextBlock.SetText` (`/Game/Ui/MainHud.CurrentXPP` (`/Game/ThirdPerson/Blueprints/BP_ThirdPersonCharacter.HudWidget` (`self.Player Character BP`))) (`|FormatText` "{CurrentXPP} {MAXXP}" (`self.XP`) (`self.MaxXP`)))
    (`ProgressBar.SetPercent` (`/Game/Ui/MainHud.DarkBar` (`/Game/ThirdPerson/Blueprints/BP_ThirdPersonCharacter.HudWidget` (`self.Player Character BP`))) (/ (`self.CurrentDark`) (`self.MaxDark`)))))

(fn `DecreaseDark`)

(fn `DecreaseHealth`
  (params (Damage :type "Float (double-precision)"))
  (returns (`IsPlayerDead?` :type Boolean))
  (if (not (<= (`self.CurrentHealth`) 0.0))
    (bind _output_get (set `self.CurrentHealth` (- (`self.CurrentHealth`) Damage)))
    (`ProgressBar.SetPercent` (select `/Game/Blueprints/E_CharacterTypes` (`self.CharacterType`) :`NewEnumerator0` (`/Game/Ui/MainHud.HealthBar` (`/Game/ThirdPerson/Blueprints/BP_ThirdPersonCharacter.HudWidget` (`self.Player Character BP`))) :`NewEnumerator1` (`/Game/Ui/WB_DummyHealthbar.HealthBar` (`/Game/Blueprints/BP_Dummy.Widget Health Ui` (`self.Dummy Blueprint`))) :`NewEnumerator2` (`/Game/Ui/WB_DummyHealthbar.HealthBar` (`/Game/AI/BP_AI.Widget Health Ui` (`self.BP AI`)))) (/ _output_get (`self.MaxHealth`)))
    (`TextBlock.SetText` (select `/Game/Blueprints/E_CharacterTypes` (`self.CharacterType`) :`NewEnumerator0` (`/Game/Ui/MainHud.HealthText` (`/Game/ThirdPerson/Blueprints/BP_ThirdPersonCharacter.HudWidget` (`self.Player Character BP`))) :`NewEnumerator1` (`/Game/Ui/WB_DummyHealthbar.HealthText` (`/Game/Blueprints/BP_Dummy.Widget Health Ui` (`self.Dummy Blueprint`))) :`NewEnumerator2` (`/Game/Ui/WB_DummyHealthbar.HealthText` (`/Game/AI/BP_AI.Widget Health Ui` (`self.BP AI`)))) (`KismetTextLibrary.Conv_DoubleToText` (`self.CurrentHealth`) "HalfToEven"))
    (if (<= (`self.CurrentHealth`) 0.0)
      _
      (else
        (return false))))
  (return true))

(fn `DecreaseStamina`
  (params (NewParam :type "Float (double-precision)"))
  (returns (NoStaminaLeft :type Boolean))
  (if (not (<= (`self.CurrentStamina`) 0.0))
    (set `self.CurrentStamina` (- (`self.CurrentStamina`) NewParam))
    (`ProgressBar.SetPercent` (`/Game/Ui/MainHud.StaminaBar` (`/Game/ThirdPerson/Blueprints/BP_ThirdPersonCharacter.HudWidget` (`self.Player Character BP`))) (/ (`self.CurrentStamina`) (`self.MaxStamina`)))
    (if (<= (`self.CurrentStamina`) 0.0)
      _
      (else
        (return false))))
  (return true))

(fn `Increase Max Health`
  (params (HealthIncrement :type "Float (double-precision)"))
  (bind _hudwidget (`/Game/ThirdPerson/Blueprints/BP_ThirdPersonCharacter.HudWidget` (`self.Player Character BP`)))
  (set `self.CurrentHealth` (+ (`self.MaxHealth`) HealthIncrement))
  (`ProgressBar.SetPercent` (`/Game/Ui/MainHud.HealthBar` _hudwidget) (/ (`self.CurrentHealth`) (`self.MaxHealth`)))
  (`TextBlock.SetText` (`/Game/Ui/MainHud.HealthText` _hudwidget) (`KismetTextLibrary.Conv_DoubleToText` (`self.CurrentHealth`) "HalfToEven")))

(fn `Increase Max Stamina`
  (params (AddStamina :type "Float (double-precision)"))
  (bind _output_get (set `self.MaxStamina` (+ (`self.MaxStamina`) AddStamina)))
  (set `self.CurrentStamina` _output_get)
  (`ProgressBar.SetPercent` (`/Game/Ui/MainHud.StaminaBar` (`/Game/ThirdPerson/Blueprints/BP_ThirdPersonCharacter.HudWidget` (`self.Player Character BP`))) (/ (`self.CurrentStamina`) (`self.MaxStamina`))))

(fn `IncreaseDark`
  (params (IncomingDark :type "Float (double-precision)" :default 5.0))
  (set `self.CurrentDark` (+ (`self.CurrentDark`) IncomingDark))
  (if (not (> (`self.CurrentDark`) (`self.MaxDark`)))
    (`ProgressBar.SetPercent` (`/Game/Ui/MainHud.DarkBar` (`/Game/ThirdPerson/Blueprints/BP_ThirdPersonCharacter.HudWidget` (`self.Player Character BP`))) (/ (`self.CurrentDark`) (`self.MaxDark`)))))

(fn `IncreaseHealth`
  (params (IncomingHealth :type "Float (double-precision)"))
  (bind _hudwidget (`/Game/ThirdPerson/Blueprints/BP_ThirdPersonCharacter.HudWidget` (`self.Player Character BP`)))
  (set `self.CurrentHealth` (+ (`self.CurrentHealth`) IncomingHealth))
  (if (> (`self.CurrentHealth`) (`self.MaxHealth`))
    (set `self.CurrentHealth` (`self.MaxHealth`)))
  (`ProgressBar.SetPercent` (`/Game/Ui/MainHud.HealthBar` _hudwidget) (/ (`self.CurrentHealth`) (`self.MaxHealth`)))
  (`TextBlock.SetText` (`/Game/Ui/MainHud.HealthText` _hudwidget) (`KismetTextLibrary.Conv_DoubleToText` (`self.CurrentHealth`) "HalfToEven")))

(fn `IncreaseLevel`
  (params (`Added Level` :type Integer))
  (set `self.Level` (+ (`self.Level`) `Added Level`))
  (set `self.MaxXP` (+ (`self.MaxXP`) 150.0))
  (set `self.XP` 0.0)
  (`TextBlock.SetText` (`/Game/Ui/MainHud.LevelText` (`/Game/ThirdPerson/Blueprints/BP_ThirdPersonCharacter.HudWidget` (`self.Player Character BP`))) (`KismetTextLibrary.Conv_IntToText` (`self.Level`)))
  (`GameplayStatics.PlaySound2D` "/Game/Audio/UI/475889__epicsoundeffects__ese-whoosh-epic-level-up.475889__epicsoundeffects__ese-whoosh-epic-level-up" 1.0 1.0 0.0 null null))

(fn `IncreaseMaxDark`)

(fn `IncreaseStamina`
  (params (IncreaseStamina :type "Float (double-precision)"))
  (set `self.CurrentStamina` (+ (`self.CurrentStamina`) IncreaseStamina))
  (if (> (`self.CurrentStamina`) (`self.MaxStamina`))
    (set `self.CurrentStamina` (`self.MaxStamina`)))
  (`ProgressBar.SetPercent` (`/Game/Ui/MainHud.StaminaBar` (`/Game/ThirdPerson/Blueprints/BP_ThirdPersonCharacter.HudWidget` (`self.Player Character BP`))) (/ (`self.CurrentStamina`) (`self.MaxStamina`))))

(fn `IncreaseXP`
  (params (`Added XP` :type "Float (double-precision)"))
  (set `self.XP` (+ (`self.XP`) `Added XP`))
  (if (>= (`self.XP`) (`self.MaxXP`))
    (`self.IncreaseLevel` 1))
  (`ProgressBar.SetPercent` (`/Game/Ui/MainHud.XPProgressBar` (`/Game/ThirdPerson/Blueprints/BP_ThirdPersonCharacter.HudWidget` (`self.Player Character BP`))) (/ (`self.XP`) (`self.MaxXP`)))
  (`TextBlock.SetText` (`/Game/Ui/MainHud.CurrentXPP` (`/Game/ThirdPerson/Blueprints/BP_ThirdPersonCharacter.HudWidget` (`self.Player Character BP`))) (`|FormatText` "{CurrentXPP} / {MAXXP}" (`self.XP`) (`self.MaxXP`))))