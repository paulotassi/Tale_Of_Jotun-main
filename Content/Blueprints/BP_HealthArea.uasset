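; Healing zone actor that restores health to a BP_ThirdPersonCharacter while it stands inside the AreaOfHealing component.
; Begin overlap stores the character and sets an in-zone flag, which end overlap clears.
; A Delay wired back into the health check forms a timed loop that calls IncreaseHealth on BPCPlayerStats until health equals max or the flag clears.
; Only one character reference and flag are stored, and each pass prints debug text.
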(event `self.AreaOfHealing.OnComponentBeginOverlap`
  (params (OverlappedComponent :type "PrimitiveComponent Object Reference") (OtherActor :type "Actor Object Reference") (OtherComp :type "PrimitiveComponent Object Reference") (OtherBodyIndex :type Integer) (bFromSweep :type Boolean) (SweepResult :type "HitResult Structure (by ref)"))
  (bind _bpc_playerstats (`/Game/ThirdPerson/Blueprints/BP_ThirdPersonCharacter.BPC_PlayerStats` (`self.As BP Third Person Character`)))
  (bind _asbp_third_person_character (cast `/Game/ThirdPerson/Blueprints/BP_ThirdPersonCharacter` OtherActor))
  (set `self.As BP Third Person Character` _asbp_third_person_character)
  (bind _output_get (set `self.IsInHealingZone?` true))
  (if _output_get
    (if (not (== (`/Game/Blueprints/BPC_PlayerStats.CurrentHealth` _bpc_playerstats) (`/Game/Blueprints/BPC_PlayerStats.MaxHealth` _bpc_playerstats))) :!label _label
      (`KismetSystemLibrary.PrintString` "Hello")
      (if (`self.IsInHealingZone?`)
        (for _ (`|MakeArray` _asbp_third_person_character)
          (`/Game/Blueprints/BPC_PlayerStats.IncreaseHealth` _bpc_playerstats 2.0)
          (`KismetSystemLibrary.Delay` 0.2)
          (goto _label))))))

(event `self.AreaOfHealing.OnComponentEndOverlap`
  (params (OverlappedComponent :type "PrimitiveComponent Object Reference") (OtherActor :type "Actor Object Reference") (OtherComp :type "PrimitiveComponent Object Reference") (OtherBodyIndex :type Integer))
  (bind _asbp_third_person_character (cast `/Game/ThirdPerson/Blueprints/BP_ThirdPersonCharacter` OtherActor))
  (set `self.As BP Third Person Character` _asbp_third_person_character)
  (set `self.IsInHealingZone?` false))

(fn `UserConstructionScript`)