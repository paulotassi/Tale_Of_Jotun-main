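; Quest giver actor that plays dialogue lines, then offers its list of quests in a UI.
; A trigger radius shows a camera-facing interact prompt while the player character overlaps it.
; Each Interact call advances the dialogue, and once the lines run out, the dialogue widget gives way to a quest widget filled from the Quests array.
; Interacting again or calling CloseWidget removes that widget and restores game-only input.
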(event `self.ReceiveTick`
  (params (DeltaSeconds :type "Float (single-precision)"))
  (`SceneComponent.K2_SetWorldRotation` (`self.InteractWidget`) (`KismetMathLibrary.FindLookAtRotation` (`SceneComponent.K2_GetComponentLocation` (`self.InteractWidget`)) (`SceneComponent.K2_GetComponentLocation` (`PlayerCameraManager.TransformComponent` (`GameplayStatics.GetPlayerCameraManager` 0)))) false false))

(event `self.TriggerRadius.OnComponentBeginOverlap`
  (params (OverlappedComponent :type "PrimitiveComponent Object Reference") (OtherActor :type "Actor Object Reference") (OtherComp :type "PrimitiveComponent Object Reference") (OtherBodyIndex :type Integer) (bFromSweep :type Boolean) (SweepResult :type "HitResult Structure (by ref)"))
  (cast `/Game/ThirdPerson/Blueprints/BP_ThirdPersonCharacter` OtherActor)
  (`SceneComponent.SetVisibility` (`self.InteractWidget`) true false))

(event `self.TriggerRadius.OnComponentEndOverlap`
  (params (OverlappedComponent :type "PrimitiveComponent Object Reference") (OtherActor :type "Actor Object Reference") (OtherComp :type "PrimitiveComponent Object Reference") (OtherBodyIndex :type Integer))
  (cast `/Game/ThirdPerson/Blueprints/BP_ThirdPersonCharacter` OtherActor)
  (`SceneComponent.SetVisibility` (`self.InteractWidget`) false false))

(event `Open Quest Widget`
  (bind _returnvalue (`|CreateWidget` "/Game/QuestsSystem/UI_QuestGiver.UI_QuestGiver_C"))
  (bind _output_get (set `self.Quest Widget` _returnvalue))
  (`UserWidget.AddToViewport` _output_get 0)
  (set `self.WidgetActive?` true)
  (set `/Game/QuestsSystem/UI_QuestGiver.QuestGiverBp` self (`self.Quest Widget`))
  (for _array_element (`self.Quests`)
    (`/Game/QuestsSystem/UI_QuestGiver.Add Quest` (`self.Quest Widget`) _array_element)))

(event `Close Widget`
  (bind _returnvalue (`GameplayStatics.GetPlayerController` 0))
  (`Widget.RemoveFromParent` (`self.Quest Widget`) :!label _label)
  (set `self.Quest Widget` null)
  (set `PlayerController.bShowMouseCursor` false _returnvalue)
  (`WidgetBlueprintLibrary.SetInputMode_GameOnly` _returnvalue)
  (set `self.WidgetActive?` false))

(event `/Game/QuestsSystem/BPI_QuestGiver.Interact`
  (bind _returnvalue (`GameplayStatics.GetPlayerController` 0))
  (if (not (`self.WidgetActive?`))
    (if (not (`self.DialougeOpen?`))
      (bind _returnvalue_2 (`|CreateWidget` "/Game/QuestsSystem/UI_QuestGiverDialougw.UI_QuestGiverDialougw_C"))
      (bind _output_get (set `self.DialougeWidget` _returnvalue_2))
      (`UserWidget.AddToViewport` _output_get 0)
      (set `self.DialougeOpen?` true)
      (`TextBlock.SetText` (`/Game/QuestsSystem/UI_QuestGiverDialougw.DialougeText` (`self.DialougeWidget`)) (`KismetTextLibrary.Conv_StringToText` (`|GetArrayItem` (`self.Dialogue`) (`self.DialougeIndex`))))
      (`/Engine/EditorBlueprintResources/StandardMacros.IncrementInt` (`self.DialougeIndex`)
        (:`  `
          (set `PlayerController.bShowMouseCursor` true _returnvalue)
          (`WidgetBlueprintLibrary.SetInputMode_GameAndUIEx` _returnvalue (`self.Quest Widget`))))
      (else
        (`TextBlock.SetText` (`/Game/QuestsSystem/UI_QuestGiverDialougw.DialougeText` (`self.DialougeWidget`)) (`KismetTextLibrary.Conv_StringToText` (`|GetArrayItem` (`self.Dialogue`) (`self.DialougeIndex`))))
        (`/Engine/EditorBlueprintResources/StandardMacros.IncrementInt` (`self.DialougeIndex`)
          (:`  `
            (if (> (`self.DialougeIndex`) (`KismetArrayLibrary.Array_Length` (`self.Dialogue`)))
              (`Widget.RemoveFromParent` (`self.DialougeWidget`))
              (set `self.DialougeWidget` null)
              (set `self.DialougeIndex` 0)
              (set `self.DialougeOpen?` false)
              (`self.Open Quest Widget`))))))
    (else
      (goto _label))))

(fn `UserConstructionScript`)