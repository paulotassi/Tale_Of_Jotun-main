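; BP_AIController_Boss is the AI controller for a boss, running the BT_AI_Boss behavior tree from BeginPlay.
; ActivateBossCombat creates a UI_BossHealthBar widget and adds it to the viewport, and DeactivateBossCombat removes it and clears the reference.
; While that widget is valid, Tick polls Health over MaxHealth to set the bar's percent.
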(event `self.ReceiveBeginPlay`
  (`self.RunBehaviorTree` "/Game/AI/Boss/BT_AI_Boss.BT_AI_Boss"))

(event `Activate Boss Combat`
  (bind _returnvalue (`|CreateWidget` "/Game/Ui/UI_BossHealthBar.UI_BossHealthBar_C"))
  (bind _output_get (set `self.Boss HealthBar Widget` _returnvalue))
  (`UserWidget.AddToViewport` _output_get 0))

(event `Deactivate Boss Combat`
  (`Widget.RemoveFromParent` (`self.Boss HealthBar Widget`))
  (set `self.Boss HealthBar Widget` null))

(event `self.ReceiveTick`
  (params (DeltaSeconds :type "Float (single-precision)"))
  (bind _boss_healthbar_widget (`self.Boss HealthBar Widget`)
    (:`then`
      (`ProgressBar.SetPercent` (`/Game/Ui/UI_BossHealthBar.HealthBar` _boss_healthbar_widget) (/ (`self.Health`) (`self.MaxHealth`))))
    (:`else`)))

(fn `UserConstructionScript`
  (`parent.UserConstructionScript`))