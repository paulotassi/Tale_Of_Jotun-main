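; BP_AI_Boss is a boss AI character Blueprint whose health is exposed to its AI controller.
; Every tick it casts its controller to BP_AIController_Boss and copies current and max health from the BPCPlayerStats component into the controller's Health and MaxHealth.
; BeginPlay and the construction script only call their parent versions, and the overlap event is disabled.
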(event `self.ReceiveBeginPlay`
  (`parent.ReceiveBeginPlay`))

(event `self.ReceiveTick`
  (params (DeltaSeconds :type "Float (single-precision)"))
  (bind _bpc_playerstats (`self.BPC_PlayerStats`))
  (`parent.ReceiveTick` DeltaSeconds)
  (bind _asbp_aicontroller_boss (cast `/Game/AI/Boss/BP_AIController_Boss` (`AIBlueprintHelperLibrary.GetAIController` self)))
  (set `/Game/AI/Boss/BP_AIController_Boss.Health` (`/Game/Blueprints/BPC_PlayerStats.CurrentHealth` _bpc_playerstats) _asbp_aicontroller_boss)
  (set `/Game/AI/Boss/BP_AIController_Boss.MaxHealth` (`/Game/Blueprints/BPC_PlayerStats.MaxHealth` _bpc_playerstats) _asbp_aicontroller_boss))

(fn `UserConstructionScript`
  (`parent.UserConstructionScript`))